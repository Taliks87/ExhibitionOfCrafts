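; BP_LessonPlace is a resizable place with a floor, four walls and a text logo, apparently a lesson area.
; Its construction script sets the logo text from LogoText and scales the floor in X and Y by Size.
; ScaleObject moves each wall outward or inward by Size and stretches its Y scale, leaving height unchanged.
; On Tick, the logo rotates to face the player camera.
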(event `self.ReceiveTick`
  (params (DeltaSeconds :type "Float (single-precision)"))
  (`AdditionalFunctionLibrary.RotateToPlayerCamera` (`self.Logo`)))

(fn `CalcScale`
  (params (Vector :type "Vector Structure"))
  (returns (ScaledVector :type "Vector Structure"))
  (bind _size (`self.Size`))
  (return (`KismetMathLibrary.MakeVector` (* Vector_X _size) (* Vector_Y _size) Vector_Z)))

(fn `ScaleObject`
  (params (Object :type "StaticMeshComponent Object Reference"))
  (bind _size (`self.Size`))
  (bind (_relativelocation_x _relativelocation_y _relativelocation_z) (`KismetMathLibrary.BreakVector` (`SceneComponent.RelativeLocation` Object)))
  (bind (_relativescale3d_x _relativescale3d_y _relativescale3d_z) (`KismetMathLibrary.BreakVector` (`SceneComponent.RelativeScale3D` Object)))
  (`SceneComponent.K2_SetRelativeLocation` Object (`KismetMathLibrary.MakeVector` (* _relativelocation_x _size) (* _relativelocation_y _size) _relativelocation_z) false false)
  (`SceneComponent.SetRelativeScale3D` Object (`KismetMathLibrary.MakeVector` _relativescale3d_x (* _relativescale3d_y (`self.Size`)) _relativescale3d_z)))

(fn `UserConstructionScript`
  (locals (NewLocalVar_0 :type Boolean :default false))
  (bind _floor (`self.Floor`))
  (`TextRenderComponent.K2_SetText` (`self.Logo`) (`self.LogoText`))
  (`SceneComponent.SetRelativeScale3D` _floor (`self.CalcScale` (`SceneComponent.RelativeScale3D` _floor)))
  (`self.ScaleObject` (`self.LeftWall`))
  (`self.ScaleObject` (`self.BackWall`))
  (`self.ScaleObject` (`self.RigthWall`))
  (`self.ScaleObject` (`self.FrontWall`)))