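; AI controller that patrols its enemy pawn along points supplied by that pawn and chases BP_Player on sight.
; Patrol cycles the points with a pause at each, retrying on failure.
; Sighting starts the chase and a short timer that clears the target and resumes patrol.
; Attack only turns the pawn toward the player and chases again; failed chases resume patrol based on a distance check.
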(event `self.ReceiveBeginPlay`
  ;[1 1 1] Init Patrol Path
  (bind _patrolpath (message `/Game/Characters/AI/Interfaces/BPI_AIPath.GetPatrolPath` (`self.K2_GetPawn`)))
  (bind _output_get (set `self.PatrolPath` _patrolpath))
  (set `self.IsCanPatrol` (`KismetArrayLibrary.Array_IsValidIndex` _output_get))
  (`self.Patrol`))

(event `Patrol`
  ;[1 1 1] Patrol
  (if (`self.IsCanPatrol`)
    (`self.Player`
      (:`then`)
      (:`else`
        (`|AIMoveTo` (`self.K2_GetPawn`) (0.0 0.0 0.0) (`|GetArrayItem` (`self.PatrolPath`) (`self.CurrentPatrolPoint`)) 50.0
          (:`OnSuccess`
            (`KismetSystemLibrary.Delay` 2.0)
            (bind _result (`/Engine/EditorBlueprintResources/StandardMacros.IncrementInt` (`self.CurrentPatrolPoint`))
              (:`  `
                (if (not (< _result (`KismetArrayLibrary.Array_Length` (`self.PatrolPath`))))
                  (set `self.CurrentPatrolPoint` 0)))))
          (:`OnFail`
            _))
        (`self.Patrol`)))))

(event `self.OnSeePawn`
  (params (Pawn :type "Pawn Object Reference"))
  ;[1 1 1] On See Pawn
  (bind _asbp_player (cast `/Game/Characters/Player/Blueprints/BP_Player` Pawn))
  (set `self.Player` _asbp_player)
  (`self.MoveToPlayer`)
  (`KismetSystemLibrary.K2_SetTimerDelegate` (delegate `Return to patrol`) 2.0))

(event `Return to patrol`
  ;[1 1 1] On See Pawn
  (set `self.Player` null)
  (`self.Patrol`))

(event `MoveToPlayer`
  ;[1 1 1] Move To Player
  (`|AIMoveTo` (`self.K2_GetPawn`) (0.0 0.0 0.0) (`self.Player`) 20.0 true
    (:`OnSuccess`
      (`self.Attack`))
    (:`OnFail`
      (bind _istoofar (`self.CheckDistanceToPlayer`))
      (if _istoofar
        (`self.Patrol`)))))

(event `Attack`
  (bind _returnvalue (`self.K2_GetPawn`))
  ;[1 1 1] Attack
  (`self.K2_SetActorRelativeRotation` _returnvalue (`KismetMathLibrary.FindLookAtRotation` (`self.K2_GetActorLocation` _returnvalue) (`self.K2_GetActorLocation` (`self.Player`))) false false)
  (`self.MoveToPlayer`))

(fn `CheckDistanceToPlayer`
  (returns (IsTooFar :type Boolean))
  (bind _returnvalue (> (`self.GetDistanceTo` (`self.K2_GetPawn`) (`self.Player`)) (`self.CriticalDistance`)))
  (if _returnvalue
    (set `self.Player` null))
  (return _returnvalue))

(fn `UserConstructionScript`)