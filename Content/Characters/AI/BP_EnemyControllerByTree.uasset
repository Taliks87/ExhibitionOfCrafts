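; Enemy AI controller that runs a behavior tree and switches enemies between patrolling and reacting to a spotted player.
; On BeginPlay it fetches the patrol path from the controlled pawn, starts the tree and sets the isCanPatrol blackboard key by whether the path has points.
; Seeing the player stores it in the Player blackboard key and sets a two-second timer that clears the key for a return to patrol.
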(event `self.ReceiveBeginPlay`
  ;[1 1 1] Init Patrol Path and Set Behavior Tree
  (bind _patrolpath (message `/Game/Characters/AI/Interfaces/BPI_AIPath.GetPatrolPath` (`self.K2_GetPawn`)))
  (set `self.PatrolPath` _patrolpath)
  (`self.RunBehaviorTree` (`self.BTAsset`))
  (`BlackboardComponent.SetValueAsBool` (`AIBlueprintHelperLibrary.GetBlackboard` null) "isCanPatrol" (`KismetArrayLibrary.Array_IsValidIndex` (`self.PatrolPath`))))

(event `/Game/Characters/AI/Interfaces/BPI_EnemyController.OnSeePawn`
  (params (Pawn :type "Pawn Object Reference"))
  ;[1 1 1] On See Pawn
  (bind _asbp_player (cast `/Game/Characters/Player/Blueprints/BP_Player` Pawn))
  (`self.SetSawPlayer` _asbp_player)
  (`KismetSystemLibrary.K2_SetTimerDelegate` (delegate `Return to patrol`) 2.0))

(event `Return to patrol`
  ;[1 1 1] On See Pawn
  (`self.SetSawPlayer` null))

(fn `SetSawPlayer`
  (params (Player :type "/Game/Characters/Player/Blueprints/BP_Player Object Reference"))
  (`BlackboardComponent.SetValueAsObject` (`AIBlueprintHelperLibrary.GetBlackboard` null) "Player" Player)
  (return))

(fn `UserConstructionScript`)