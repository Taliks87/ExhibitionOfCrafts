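; Base NPC Blueprint that shows a floating name label and provides default focus and interaction responses.
; The construction script fills the label from NPCName, and OnFriendlyChange colors it green or red by friendliness, first applied at BeginPlay.
; Tick keeps the label turned toward the player camera.
; OnFocus prints a talk prompt with the bound Interact key, while Interact prints a placeholder reply.
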(event `self.ReceiveBeginPlay`
  (`self.OnFriendlyChange` (`self.IsFriendly`)))

(event `self.ReceiveTick`
  (params (DeltaSeconds :type "Float (single-precision)"))
  (`AdditionalFunctionLibrary.RotateToPlayerCamera` (`self.TextName`)))

(event `/Game/Base/Interfaces/BPI_Interact.OnFocus`
  ;[1 1 1] Base Focus and Interaction
  (bind _returnvalue (`AdditionalFunctionLibrary.GetActionPrimaryKeyName` "Interact"))
  (`KismetSystemLibrary.PrintString` (`KismetTextLibrary.Conv_TextToString` (`|FormatText` "Press \"{1}\" for Talk" _returnvalue))))

(event `/Game/Base/Interfaces/BPI_Interact.Interact`
  (params (Character :type "Character Object Reference"))
  ;[1 1 1] Base Focus and Interaction
  (`KismetSystemLibrary.PrintString` "Nothing to say. Bye!"))

(fn `OnFriendlyChange`
  (params (Condition :type Boolean))
  (bind _textname (`self.TextName`))
  (bind _output_get (set `self.IsFriendly` Condition))
  (if _output_get
    (`TextRenderComponent.SetTextRenderColor` _textname (make `Color` 0 255 0 255))
    (else
      (`TextRenderComponent.SetTextRenderColor` _textname (make `Color` 0 0 255 255)))))

(fn `UserConstructionScript`
  (`TextRenderComponent.K2_SetText` (`self.TextName`) (`self.NPCName`)))