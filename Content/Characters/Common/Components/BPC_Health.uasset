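; BPC_Health is a health component for characters that tracks current health against a maximum and starts full on BeginPlay.
; AddHealth, FillHealth and TakeDamage change the value, capping healing at the maximum and damage at zero, then fire the health-change event dispatcher.
; TakeDamage also fires the died dispatcher whenever a positive hit leaves health at zero, including hits after death.
; GetHealth and IsDied expose the current state.
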(event `self.ReceiveBeginPlay`
  (set `self.Health` (`self.MaxHealt`)))

(fn `AddHealth`
  (params (Health :type "Float (double-precision)"))
  (bind _maxhealt (`self.MaxHealt`))
  (if (> Health 0.0)
    (bind _output_get (set `self.Health` (+ Health (`self.Health`))))
    (if (> _output_get _maxhealt)
      (set `self.Health` _maxhealt))
    (`self.ED_OnHealthChange`)))

(fn `FillHealth`
  (set `self.Health` (`self.MaxHealt`))
  (`self.ED_OnHealthChange`))

(fn `GetHealth`
  (returns (Health :type "Float (double-precision)"))
  (return (`self.Health`)))

(fn `IsDied`
  (returns (IsDied :type Boolean))
  (return (== (`self.Health`) 0.0)))

(fn `TakeDamage`
  (params (Damage :type "Float (double-precision)"))
  (if (> Damage 0.0)
    (bind _output_get (set `self.Health` (- (`self.Health`) Damage)))
    (if (<= _output_get 0.0)
      (set `self.Health` 0.0)
      (`self.ED_OnDied`))
    (`self.ED_OnHealthChange`)))