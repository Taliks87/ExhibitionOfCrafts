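; BP_Enemy is an enemy character Blueprint that sets itself unfriendly on BeginPlay.
; Its PawnSensing component forwards seen pawns to the controller through the BPI_EnemyController interface, leaving the response to the controller.
; It also exposes its PatrolPath through a GetPatrolPath getter.
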(event `self.ReceiveBeginPlay`
  ;[1 1 1] Init unfriendly
  (`parent.ReceiveBeginPlay`)
  (`self.SetFriendly` false))

(event `self.PawnSensing.OnSeePawn`
  (params (Pawn :type "Pawn Object Reference"))
  ;[1 1 1] On See Pawn
  (bind _asbpi_enemy_controller (cast `/Game/Characters/AI/Interfaces/BPI_EnemyController` (`self.GetController`)))
  (`/Game/Characters/AI/Interfaces/BPI_EnemyController.OnSeePawn` _asbpi_enemy_controller Pawn))

(fn `GetPatrolPath`
  (returns (PatrolPath :type "Array of TargetPoint Object Reference"))
  (return (`self.PatrolPath`)))

(fn `UserConstructionScript`
  (`parent.UserConstructionScript`))