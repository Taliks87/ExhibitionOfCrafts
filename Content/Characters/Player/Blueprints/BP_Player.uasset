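; BP_Player is the player character Blueprint that detects and interacts with objects through the BPI_Interact interface.
; Each tick, a short sphere trace from the actor's location along the follow camera's forward vector finds WorldDynamic or Pawn objects.
; When the hit changes, the previous focus is notified of losing focus and any interactable hit gains it.
; Pressing Interact sends an interact message to the focused object, passing the player.
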(event `self.ReceiveTick`
  (params (DeltaSeconds :type "Float (single-precision)"))
  (`self.RefreshObjectInFocus`))

(event `InputAction|Interact`
  (params (Key :type "Key Structure"))
  (:`Pressed`
    (`self.InteractWithObject`)))

(fn `InteractWithObject`
  (bind _returnvalue (`KismetSystemLibrary.Conv_InterfaceToObject` (`self.ObjectInFocus`)))
  (`/Engine/EditorBlueprintResources/StandardMacros.IsValid` _returnvalue
    (:`Is Valid`
      (message `/Game/Base/Interfaces/BPI_Interact.Interact` _returnvalue self))))

(fn `RefreshObjectInFocus`
  (bind _returnvalue (`self.K2_GetActorLocation` self))
  (bind _returnvalue_2 (`KismetSystemLibrary.Conv_InterfaceToObject` (`self.ObjectInFocus`)))
  (bind _outhit (`KismetSystemLibrary.SphereTraceSingleForObjects` _returnvalue (+ _returnvalue (* (`SceneComponent.GetForwardVector` (`self.FollowCamera`)) 130.0)) 20.0 (`|MakeArray` "ObjectTypeQuery2" "ObjectTypeQuery3" :!type "EObjectTypeQuery Enum")))
  (if (!= _returnvalue_2 (`.HitActor` (`GameplayStatics.BreakHitResult` _outhit)))
    (`/Engine/EditorBlueprintResources/StandardMacros.IsValid` _returnvalue_2
      (:`Is Valid`
        (message `/Game/Base/Interfaces/BPI_Interact.OnLostFocus` _returnvalue_2)
        (set `self.ObjectInFocus` null))
      (:`Is Not Valid`
        _))
    (bind _asbpi_interact (cast `/Game/Base/Interfaces/BPI_Interact` (`.HitActor` (`GameplayStatics.BreakHitResult` _outhit))))
    (bind _output_get (set `self.ObjectInFocus` _asbpi_interact))
    (`/Game/Characters/Common/Blueprints/BP_NPCBase.OnFocus` _output_get)))

(fn `UserConstructionScript`)